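; BP_PlayerCharacter is the player character Blueprint, handling pickup interaction, weapon swapping and an idler-game UI.
; E sends InteractMessage to the first overlapping BP_PickUpMaster, while key 1 opens PlayerUI_BP with UI-only input.
; SpawnWeapon drops the current weapon as its pickup class, then adds the new weapon as a component on its mesh socket.
; Mouse buttons hold basic logged spawn and destroy calls, the latter destroying the character itself.
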(event Custom|Spawn%20Weapon
  (params (Weapon%20To%20Spawn :type BP%20Weapon%20Master%20Class%20Reference) (Pickups%20Location :type Vector))
  (bind _current_weapon (Variables|Default|GetCurrent%20Weapon)
    (:then
      (Game|SpawnActorfromClass (Variables|/Game/MyStuff/FPSPlayer/Weapons/BP_WeaponMaster.BP_WeaponMaster_C|GetPickupClass _current_weapon) (Math|Transform|MakeTransform (+ Pickups%20Location "0.000000,0.000000,10.000000") "0, 0, 0" "1.000000,1.000000,1.000000") "AdjustIfPossibleButAlwaysSpawn" "MultiplyWithRoot" 0 0)
      (Components|DestroyComponent _current_weapon))
    (:else
      _))
  (bind _returnvalue (Game|AddComponentbyClass Weapon%20To%20Spawn false))
  (bind _output_get (Variables|Default|SetCurrent%20Weapon _returnvalue))
  (Transformation|AttachComponentToComponent _output_get (Variables|Character|GetMesh) (Variables|/Game/MyStuff/FPSPlayer/Weapons/BP_WeaponMaster.BP_WeaponMaster_C|GetSocketName _output_get) "SnapToTarget" "SnapToTarget" "SnapToTarget" true)
  (Development|PrintText "PickedUp"))

(event EventBeginPlay)

(event Collision|EventActorBeginOverlap
  (params (OtherActor :type Actor%20Object%20Reference)))

(event EventTick
  (params (DeltaSeconds :type Float%20%28single-precision%29)))

(event Input|MouseEvents|LeftMouseButton
  (params (Key :type Key%20Structure :default "None"))
  ;[0.15 0.15 0.15 0.5] Spawning Methods
  (:Pressed
    (Class|PlayerCharacter|SpawnActor)
    (Utilities|String|LogString "Spawned Actor")))

(event Input|MouseEvents|RightMouseButton
  (params (Key :type Key%20Structure :default "None"))
  ;[0.15 0.15 0.15 0.5] Spawning Methods
  (:Pressed
    (Class|PlayerCharacter|DestroyActor)
    (Utilities|String|LogString "Destroying Actor")))

(event Input|KeyboardEvents|1
  (params (Key :type Key%20Structure :default "None"))
  ;[0.15 0.15 0.15 0.5] Idler Game
  (:Pressed
    (bind _returnvalue (UserInterface|CreateWidget "/Game/MyStuff/Idler/PlayerUI_BP.PlayerUI_BP_C"))
    (UserInterface|Viewport|AddtoViewport _returnvalue 0)
    (bind _asplayer_controller (Utilities|Casting|CastToPlayerController (Game|GetPlayerController 0)))
    (Input|SetInputModeUIOnly _asplayer_controller _returnvalue "DoNotLock" false)))

(event Input|KeyboardEvents|E
  (params (Key :type Key%20Structure :default "None"))
  (:Pressed
    (Class|BPIInteract|Interact(Message) (Utilities|Array|Get(acopy) (Collision|GetOverlappingActors "/Game/MyStuff/FPSPlayer/Pickups/BP_PickUpMaster.BP_PickUpMaster_C" :!class /Script/Engine.Actor)) self)))

(fn ConstructionScript)